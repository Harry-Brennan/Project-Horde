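; Base enemy Blueprint that faces the player, fires at them if ranged, and takes damage until death.
; On BeginPlay it plays a spawn effect, then loads stats, emitters and projectile from DT_Classes by ClassName.
; A looping aim timer yaws the mesh and, for ranged enemies within a distance band, starts or clears a looping shoot timer.
; Spawning, shooting, damage and death are delegated to components, with brief invincibility following each hit.
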(event Custom|ShootLoop
  (Default|Shoot (Variables|Default|GetBPC_Shoot) (Variables|INFO|GetBase%20Projectile) (Variables|Character|GetMesh) (Game|GetPlayerCharacter 0)))

(event Custom|AimAtEnemy
  (bind _returnvalue (Game|GetPlayerCharacter 0))
  (bind _returnvalue_2 (Transformation|GetActorLocation))
  (bind _returnvalue_3 (Transformation|GetActorLocation _returnvalue))
  (bind _returnvalue_4 (Math|Vector|Distance(Vector) _returnvalue_3 _returnvalue_2))
  (Transformation|SetWorldRotation (Variables|Character|GetMesh) (Math|Rotator|MakeRotator 0.0 0.0 (+ (.yaw (Math|Rotator|FindLookatRotation _returnvalue_2 _returnvalue_3)) 2.7e+02)) false false)
  (if (and (Variables|INFO|GetRanged?) (and (< _returnvalue_4 2.5e+03) (> _returnvalue_4 2.5e+02)))
    (Utilities|FlowControl|DoOnce false :!label _label
      (:Completed
        (bind _returnvalue_5 (Utilities|Time|SetTimerbyEvent (delegate Custom|ShootLoop) (Variables|INFO|GetReload%20Speed) true))))
    (else
      (Utilities|Time|ClearandInvalidateTimerbyHandle _returnvalue_5)
      (goto _label Reset))))

(event EventTakeDamage
  (params (DamageToTake :type Float%20%28double-precision%29))
  (bind _health (Default|TakeDamage (Variables|Default|GetBPC_Take_Damage) (Variables|INFO|GetHealth) DamageToTake (not (Variables|TakingDamage|GetInvincible))))
  (Utilities|FlowControl|Sequence
    (:then_0
      (if (<= _health 0.0)
        (Default|Death (Variables|Default|GetBPC_Death) (Variables|Character|GetMesh))
        (else
          (Variables|INFO|SetHealth _health))))
    (:then_1
      (Variables|TakingDamage|SetInvincible true)
      (Utilities|FlowControl|Delay 0.2)
      (Variables|TakingDamage|SetInvincible false))))

(event EventUpdateINFO
  (CallFunction|UpdateINFOFunc))

(event EventBeginPlay
  (Utilities|FlowControl|Sequence
    (:then_0
      (Default|SpawninEffect (Variables|Default|GetBPC_Spawn) (Variables|INFO|GetSpawnInEmitter)))
    (:then_1
      (CallFunction|UpdateINFO))
    (:then_2
      (Utilities|Time|SetTimerbyEvent (delegate Custom|AimAtEnemy) 0.1 true))))

(fn ConstructionScript)

(fn UpdateINFOFunc
  (bind _returnvalue (Utilities|GetDataTableRow "/Game/Structs_DataTables/DT_Classes.DT_Classes" (Variables|INFO|GetClassName))
    (:then
      (Variables|INFO|SetHealth (.Health (Utilities|Struct|BreakStruct_Classes _returnvalue)))
      (Variables|INFO|SetSpeed (.Speed (Utilities|Struct|BreakStruct_Classes _returnvalue)))
      (Variables|INFO|SetBase%20Damage (.BaseDamage (Utilities|Struct|BreakStruct_Classes _returnvalue)))
      (Variables|INFO|SetBase%20Armour (.BaseArmour (Utilities|Struct|BreakStruct_Classes _returnvalue)))
      (Variables|INFO|SetSpawnInEmitter (.SpawnInEmitter (Utilities|Struct|BreakStruct_Classes _returnvalue)))
      (Variables|INFO|SetDeath%20Emitter (.DeathEmitter (Utilities|Struct|BreakStruct_Classes _returnvalue)))
      (Variables|INFO|SetRanged? (.Ranged? (Utilities|Struct|BreakStruct_Classes _returnvalue)))
      (Variables|INFO|SetReload%20Speed (.ReloadSpeed (Utilities|Struct|BreakStruct_Classes _returnvalue)))
      (Variables|INFO|SetBase%20Projectile (.BaseProjectile (Utilities|Struct|BreakStruct_Classes _returnvalue))))))