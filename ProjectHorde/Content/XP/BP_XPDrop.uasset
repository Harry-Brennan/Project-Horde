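; BP_XPDrop is an XP pickup that grants XP to a BPI_Player actor when its mesh overlaps it, then destroys itself.
; On BeginPlay it reads its XP amount and material from DT_XP_Types by type name.
; Entering MagnetismDetection starts a looping distance check against the player's magnetism range; once in range, a short timer plays a timeline that lerps the drop toward the player.
; Leaving detection clears both timers.
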(event OnComponentBeginOverlap(StaticMesh)
  (params (OverlappedComponent :type Primitive%20Component%20Object%20Reference) (OtherActor :type Actor%20Object%20Reference) (OtherComp :type Primitive%20Component%20Object%20Reference) (OtherBodyIndex :type Integer) (bFromSweep :type Boolean) (SweepResult :type Hit%20Result%20Structure%20%28by%20ref%29))
  (if (Utilities|DoesObjectImplementInterface OtherActor "/Game/Player/BPI_Player.BPI_Player_C")
    (Class|BPIPlayer|AddXP(Message) OtherActor (Variables|Default|GetXPTo%20Give))
    (Utilities|Time|ClearandInvalidateTimerbyHandle (Variables|Default|GetMagnetismTimer))
    (Utilities|Time|ClearandInvalidateTimerbyHandle (Variables|Default|GetCheckDistanceToPlayerTimer))
    (Actor|DestroyActor)))

(event OnComponentBeginOverlap(MagnetismDetection)
  (params (OverlappedComponent :type Primitive%20Component%20Object%20Reference) (OtherActor :type Actor%20Object%20Reference) (OtherComp :type Primitive%20Component%20Object%20Reference) (OtherBodyIndex :type Integer) (bFromSweep :type Boolean) (SweepResult :type Hit%20Result%20Structure%20%28by%20ref%29))
  (if (Utilities|DoesObjectImplementInterface OtherActor "/Game/Player/BPI_Player.BPI_Player_C")
    (bind _xpmagnetismrange (Class|BPIPlayer|GetXPMagnetismRange(Message) (Game|GetPlayerCharacter 0)))
    (bind _returnvalue (Utilities|Time|SetTimerbyEvent (delegate Custom|CheckDistanceToPlayer) 0.5 true))
    (Variables|Default|SetCheckDistanceToPlayerTimer _returnvalue)))

(event OnComponentEndOverlap(MagnetismDetection)
  (params (OverlappedComponent :type Primitive%20Component%20Object%20Reference) (OtherActor :type Actor%20Object%20Reference) (OtherComp :type Primitive%20Component%20Object%20Reference) (OtherBodyIndex :type Integer))
  (if (Utilities|DoesObjectImplementInterface OtherActor "/Game/Player/BPI_Player.BPI_Player_C")
    (Utilities|Time|ClearandInvalidateTimerbyHandle (Variables|Default|GetMagnetismTimer))
    (Utilities|Time|ClearandInvalidateTimerbyHandle (Variables|Default|GetCheckDistanceToPlayerTimer))))

(event Custom|MagnetismToPlayer
  (bind _alpha (Timeline|Alpha Play)
    (:Update
      (Transformation|SetActorLocation (Math|Vector|Lerp(Vector) (Transformation|GetActorLocation) (Transformation|GetActorLocation (Game|GetPlayerCharacter 0)) _alpha) false false))))

(event Custom|CheckDistanceToPlayer
  (if (< (Math|Vector|Distance(Vector) (Transformation|GetActorLocation) (Transformation|GetActorLocation (Game|GetPlayerCharacter 0))) (stale OnComponentBeginOverlap(MagnetismDetection) _xpmagnetismrange))
    (bind _returnvalue (Utilities|Time|SetTimerbyEvent (delegate Custom|MagnetismToPlayer) 0.1))
    (Variables|Default|SetMagnetismTimer _returnvalue)
    (Utilities|Time|ClearandInvalidateTimerbyHandle (Variables|Default|GetCheckDistanceToPlayerTimer))))

(event EventBeginPlay
  (CallFunction|UpdateINFO))

(fn ConstructionScript)

(fn UpdateINFO
  (bind _returnvalue (Utilities|GetDataTableRow "/Game/Structs_DataTables/DT_XP_Types.DT_XP_Types" (Variables|Default|GetXPTypeName))
    (:then
      (Variables|Default|SetXPTo%20Give (.XPToGive (Utilities|Struct|BreakStruct_XP_Types _returnvalue)))
      (Rendering|Material|SetMaterial (Variables|Default|GetStaticMesh) 0 (.Material (Utilities|Struct|BreakStruct_XP_Types _returnvalue))))))