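; Projectile actor that damages players or enemies on overlap, configured per row of DT_Projectiles.
; The construction script calls UpdateINFO, which loads speed, damage, piercing and mesh from the row matching Name.
; Mesh overlaps ignore enemy detection collision and use interface checks: player-owned shots hurt enemies, all others hurt players.
; Non-piercing projectiles destroy themselves after dealing damage.
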(event OnComponentBeginOverlap(ProjectileStaticMesh)
  (params (OverlappedComponent :type Primitive%20Component%20Object%20Reference) (OtherActor :type Actor%20Object%20Reference) (OtherComp :type Primitive%20Component%20Object%20Reference) (OtherBodyIndex :type Integer) (bFromSweep :type Boolean) (SweepResult :type Hit%20Result%20Structure%20%28by%20ref%29))
  (bind _piercing_ (Variables|Default|GetPiercing?))
  (bind _collisionref (Class|BPIPlayer|GetEnemyDetectionCollisionRef(Message) OtherActor))
  (if (not (== _collisionref OtherComp))
    (if (Utilities|DoesObjectImplementInterface (Components|GetOwner) "/Game/Player/BPI_Player.BPI_Player_C")
      (if (Utilities|DoesObjectImplementInterface OtherActor "/Game/Enemies/BPI_Enemy.BPI_Enemy_C")
        (Class|BPIEnemy|TakeDamage(Message) OtherActor (Variables|Default|GetBase%20Damage))
        (if (not _piercing_)
          (Actor|DestroyActor :!label _label)))
      (elif (Utilities|DoesObjectImplementInterface OtherActor "/Game/Player/BPI_Player.BPI_Player_C")
        (Class|BPIPlayer|TakeDamage(Message) OtherActor (Variables|Default|GetBase%20Damage))
        (if (not _piercing_)
          (goto _label))))))

(event EventBeginPlay)

(event Collision|EventActorBeginOverlap
  (params (OtherActor :type Actor%20Object%20Reference)))

(event EventTick
  (params (DeltaSeconds :type Float%20%28single-precision%29)))

(event EventUpdateINFO
  (bind _returnvalue (Utilities|GetDataTableRow "/Game/Structs_DataTables/DT_Projectiles.DT_Projectiles" (Variables|Default|GetName))
    (:then
      (bind _output_get (Variables|Default|SetBase%20Speed (.BaseSpeed (Utilities|Struct|BreakStruct_Projectiles _returnvalue))))
      (Variables|/Script/Engine.ProjectileMovementComponent|SetInitialSpeed (Variables|Default|GetProjectileMovement) _output_get)
      (Variables|Default|SetBase%20Damage (.BaseDamage (Utilities|Struct|BreakStruct_Projectiles _returnvalue)))
      (Variables|Default|SetPiercing? (.Piercing? (Utilities|Struct|BreakStruct_Projectiles _returnvalue)))
      (bind _output_get_2 (Variables|Default|SetStatic%20Mesh (.StaticMesh (Utilities|Struct|BreakStruct_Projectiles _returnvalue))))
      (Components|StaticMesh|SetStaticMesh (Variables|Default|GetProjectileStaticMesh) _output_get_2))))

(fn ConstructionScript
  (CallFunction|UpdateINFO))