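; Area-of-effect zone actor that applies a damage-over-time status to opposing characters standing inside it, then destroys itself after a set duration.
; On BeginPlay it loads damage, duration, status and colour from DT_AOEEffects, then sizes the detection sphere and scales the mesh to the altered radius.
; Overlap begin and end send start and stop DOT messages, using BPI_Player and BPI_Enemy checks on owner and target to pick sides.
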(event OnComponentBeginOverlap(HitDetection)
  (params (OverlappedComponent :type Primitive%20Component%20Object%20Reference) (OtherActor :type Actor%20Object%20Reference) (OtherComp :type Primitive%20Component%20Object%20Reference) (OtherBodyIndex :type Integer) (bFromSweep :type Boolean) (SweepResult :type Hit%20Result%20Structure%20%28by%20ref%29))
  (bind _returnvalue (Components|GetOwner))
  (bind _status_effect (Variables|Default|GetStatus%20Effect))
  (bind _base_damage (Variables|Default|GetBase%20Damage))
  (if (Utilities|DoesObjectImplementInterface (Components|GetOwner) "/Game/Player/BPI_Player.BPI_Player_C")
    (if (Utilities|DoesObjectImplementInterface OtherActor "/Game/Enemies/BPI_Enemy.BPI_Enemy_C")
      (Class|BPIEnemy|Start/StopDOT(Message) OtherActor _status_effect true _base_damage _returnvalue))
    (elif (Utilities|DoesObjectImplementInterface OtherActor "/Game/Player/BPI_Player.BPI_Player_C")
      (Class|BPIPlayer|Start/StopDOT(Message) OtherActor _status_effect true _base_damage _returnvalue))))

(event OnComponentEndOverlap(HitDetection)
  (params (OverlappedComponent :type Primitive%20Component%20Object%20Reference) (OtherActor :type Actor%20Object%20Reference) (OtherComp :type Primitive%20Component%20Object%20Reference) (OtherBodyIndex :type Integer))
  (bind _returnvalue (Components|GetOwner))
  (bind _status_effect (Variables|Default|GetStatus%20Effect))
  (bind _base_damage (Variables|Default|GetBase%20Damage))
  (if (Utilities|DoesObjectImplementInterface (Components|GetOwner) "/Game/Player/BPI_Player.BPI_Player_C")
    (if (Utilities|DoesObjectImplementInterface OtherActor "/Game/Enemies/BPI_Enemy.BPI_Enemy_C")
      (Class|BPIEnemy|Start/StopDOT(Message) OtherActor _status_effect false _base_damage _returnvalue))
    (elif (Utilities|DoesObjectImplementInterface OtherActor "/Game/Player/BPI_Player.BPI_Player_C")
      (Class|BPIPlayer|Start/StopDOT(Message) OtherActor _status_effect false _base_damage _returnvalue))))

(event Custom|StartTimerForLifetime
  (Actor|DestroyActor))

(event EventBeginPlay
  (bind _aoestaticmesh (Variables|Default|GetAOEStaticMesh))
  (bind _returnvalue (Transformation|GetRelativeTransform _aoestaticmesh))
  (bind _returnvalue_2 (Utilities|GetDataTableRow "/Game/Structs_DataTables/DT_AOEEffects.DT_AOEEffects" (Variables|Default|GetName))
    (:then
      (Variables|Default|SetBase%20Damage (.BaseDamage (Utilities|Struct|BreakStruct_AOEEffects _returnvalue_2)))
      (Variables|Default|SetDuration (.Duration (Utilities|Struct|BreakStruct_AOEEffects _returnvalue_2)))
      (Variables|Default|SetStatus%20Effect (.StatusEffect (Utilities|Struct|BreakStruct_AOEEffects _returnvalue_2)))
      (Variables|Default|SetColour (.Colour (Utilities|Struct|BreakStruct_AOEEffects _returnvalue_2)))
      (Components|Sphere|SetSphereRadius (Variables|Default|GetHitDetection) (Variables|Default|GetAlteredAOERadius) true)
      (Transformation|SetRelativeTransform _aoestaticmesh (Math|Transform|MakeTransform (.location _returnvalue) (.rotation _returnvalue) (* (.scale _returnvalue) (/ (Variables|Default|GetAlteredAOERadius) (.BaseAOERadius (Utilities|Struct|BreakStruct_AOEEffects _returnvalue_2))))) false false)
      (Utilities|Time|SetTimerbyEvent (delegate Custom|StartTimerForLifetime) (Variables|Default|GetDuration)))))

(fn ConstructionScript)