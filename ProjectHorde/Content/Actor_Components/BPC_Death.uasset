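; Actor component that handles death for both the player and other characters through a single Death function.
; It hides the mesh, disables collision, spawns the death emitter, clears attack and aim timers, and stops movement.
; Owners implementing BPI_Player get a cached Game Over widget with UI-only input and a mouse cursor.
; Other owners scatter BP_XPDrop pickups, splitting their XP greedily into large, medium and small drops.
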(event EventBeginPlay)

(event EventTick
  (params (DeltaSeconds :type Float%20%28single-precision%29)))

(fn Death
  (params (Mesh :type Skeletal%20Mesh%20Component%20Object%20Reference) (DeathEmitter :type Particle%20System%20Object%20Reference) (RangedAttackTimer :type Timer%20Handle%20Structure) (MeleeAttackTimer :type Timer%20Handle%20Structure) (AimTimer :type Timer%20Handle%20Structure) (Character%20Movement :type Character%20Movement%20Component%20Object%20Reference) (XPToGive :type Float%20%28double-precision%29))
  (bind _returnvalue (Components|GetOwner))
  (bind _returnvalue_2 (Game|GetPlayerController 0))
  (bind _returnvalue_3 (Math|Random|RandomFloatinRange 0.0 5.0))
  (bind _returnvalue_4 (Math|Random|RandomFloatinRange 0.0 5.0))
  (bind _returnvalue_5 (Transformation|GetActorLocation _returnvalue))
  (bind _returnvalue_6 (+ (.x _returnvalue_5) _returnvalue_4))
  (bind _returnvalue_7 (+ (.y _returnvalue_5) _returnvalue_3))
  (Rendering|SetVisibility Mesh false false)
  (Collision|SetActorEnableCollision (Components|GetOwner) false)
  (bind _returnvalue_8 (Effects|SpawnEmitteratLocation DeathEmitter (Transformation|GetActorLocation (Components|GetOwner))))
  (Utilities|Time|ClearandInvalidateTimerbyHandle RangedAttackTimer)
  (Utilities|Time|ClearandInvalidateTimerbyHandle MeleeAttackTimer)
  (Utilities|Time|ClearandInvalidateTimerbyHandle AimTimer)
  (Components|Movement|StopMovementImmediately Character%20Movement)
  (if (Utilities|DoesObjectImplementInterface _returnvalue "/Game/Player/BPI_Player.BPI_Player_C")
    (Utilities|IsValid (LocalVariables|GetGameOverScreenRef)
      (:Is%20Valid
        _)
      (:Is%20Not%20Valid
        (bind _returnvalue_9 (UserInterface|CreateWidget "/Game/UI/WBP_GameOver.WBP_GameOver_C"))
        (LocalVariables|SetGameOverScreenRef _returnvalue_9)))
    (UserInterface|Viewport|AddtoViewport (LocalVariables|GetGameOverScreenRef) 0)
    (Input|SetInputModeUIOnly _returnvalue_2 (LocalVariables|GetGameOverScreenRef) "DoNotLock" false)
    (Input|SetIgnoreMoveInput _returnvalue_2 false)
    (Development|PrintString "ATTEMPTED TO ADD GAME OVER SCREEN")
    (Variables|/Script/Engine.PlayerController|SetbShowMouseCursor _returnvalue_2 true)
    (else
      (LocalVariables|SetXP XPToGive)
      (for _index (range 1 (/ XPToGive 50))
        (Game|SpawnActorfromClass "/Game/XP/BP_XPDrop.BP_XPDrop_C" (Math|Transform|MakeTransform (Math|Vector|MakeVector _returnvalue_6 _returnvalue_7 (.z _returnvalue_5)) "0, 0, 0" "1.000000,1.000000,1.000000") "AdjustIfPossibleButAlwaysSpawn" "MultiplyWithRoot" 0 "Large" 0)
        (LocalVariables|SetXP (- (LocalVariables|GetXP) 5e+01)))
      (for _index_2 (range 1 (/ (LocalVariables|GetXP) 25))
        (Game|SpawnActorfromClass "/Game/XP/BP_XPDrop.BP_XPDrop_C" (Math|Transform|MakeTransform (Math|Vector|MakeVector _returnvalue_6 _returnvalue_7 (.z _returnvalue_5)) "0, 0, 0" "1.000000,1.000000,1.000000") "AdjustIfPossibleButAlwaysSpawn" "MultiplyWithRoot" 0 "Medium" 0)
        (LocalVariables|SetXP (- (LocalVariables|GetXP) 25.0)))
      (for _index_3 (range 1 (/ (LocalVariables|GetXP) 10))
        (Game|SpawnActorfromClass "/Game/XP/BP_XPDrop.BP_XPDrop_C" (Math|Transform|MakeTransform (Math|Vector|MakeVector _returnvalue_6 _returnvalue_7 (.z _returnvalue_5)) "0, 0, 0" "1.000000,1.000000,1.000000") "AdjustIfPossibleButAlwaysSpawn" "MultiplyWithRoot" 0 "Small" 0)
        (LocalVariables|SetXP (- (LocalVariables|GetXP) 1e+01)))
      (return _returnvalue_8))))