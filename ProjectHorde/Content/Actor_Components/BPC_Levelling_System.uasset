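; Actor component that tracks XP and level and triggers an upgrade choice on level-up.
; AddXP carries overflow past the threshold into one LevelUp call, which increments the level and raises the requirement by a level-scaled amount.
; LevelUp lazily creates and reuses the ability power choice widget, sets UI-only input with a visible cursor, freezes gameplay via zero global time dilation, then populates upgrades.
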(event EventBeginPlay)

(event EventTick
  (params (DeltaSeconds :type Float%20%28single-precision%29)))

(fn AddXP
  (params (XPToAdd :type Float%20%28double-precision%29))
  (bind _xptolevel (Variables|Default|GetXPToLevel))
  (if (>= (+ (Variables|Default|GetCurrentXP) XPToAdd) _xptolevel)
    (Variables|Default|SetCurrentXP (- (+ (Variables|Default|GetCurrentXP) XPToAdd) _xptolevel))
    (CallFunction|LevelUp)
    (else
      (Variables|Default|SetCurrentXP (+ (Variables|Default|GetCurrentXP) XPToAdd)))))

(fn LevelUp
  (bind _returnvalue (Game|GetPlayerController 0))
  (bind _currentlevel (Variables|Default|GetCurrentLevel))
  (Math|Integer|IncrementInt _currentlevel
    (:%20%20
      (Variables|Default|SetXPToLevel (+ (Variables|Default|GetXPToLevel) (* _currentlevel 10)))
      (Utilities|IsValid (LocalVariables|GetAbilityPowerChoiceRef)
        (:Is%20Valid
          _)
        (:Is%20Not%20Valid
          (bind _returnvalue_2 (UserInterface|CreateWidget "/Game/UI/WBP_Ability_Power_Choice.WBP_Ability_Power_Choice_C"))
          (LocalVariables|SetAbilityPowerChoiceRef _returnvalue_2)))
      (UserInterface|Viewport|AddtoViewport (LocalVariables|GetAbilityPowerChoiceRef) 0)
      (Variables|/Script/Engine.PlayerController|SetbShowMouseCursor _returnvalue true)
      (Input|SetInputModeUIOnly _returnvalue (LocalVariables|GetAbilityPowerChoiceRef) "DoNotLock" false)
      (Utilities|Time|SetGlobalTimeDilation 0.0)
      (Default|PopulateUpgrades (LocalVariables|GetAbilityPowerChoiceRef)))))