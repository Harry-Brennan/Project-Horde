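; Actor component that applies damage over time to its owning actor from an area effect.
; StartDOT stores the effect settings, ticks immediately, then loops on a timer until StopDOT clears it.
; Each tick sends damage, passing the effect name for BPI_Player sources, with Leeched healing the effect owner and Slowed halving walk speed again.
; StopDOT raises walk speed by half only for Ice, not Slowed.
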(event Custom|StopDOT
  (bind _movement_component (Variables|Default|GetMovement%20Component))
  (Utilities|Time|ClearandInvalidateTimerbyHandle (Variables|Default|GetDOTTimer))
  (switch name (Variables|Default|GetEffectName)
    (:Ice
      (Variables|/Script/Engine.CharacterMovementComponent|SetMaxWalkSpeed _movement_component (* (Variables|/Script/Engine.CharacterMovementComponent|GetMaxWalkSpeed _movement_component) 1.5)))))

(event Custom|StartDOT
  (params (DOTDamage :type Float%20%28double-precision%29) (EffectName :type Name) (MovementComponent :type Character%20Movement%20Component%20Object%20Reference) (AOEEffectOwner :type Actor%20Object%20Reference))
  (Variables|Default|SetDOTDamage DOTDamage)
  (Variables|Default|SetEffectName EffectName)
  (Variables|Default|SetMovement%20Component MovementComponent)
  (CallFunction|DOTDamageTick)
  (bind _returnvalue (Utilities|Time|SetTimerbyEvent (delegate Custom|DOTDamageTick) (Variables|Default|GetDOTTick) true))
  (Variables|Default|SetDOTTimer _returnvalue))

(event Custom|DOTDamageTick
  (bind _returnvalue (Components|GetOwner))
  (bind _movement_component (Variables|Default|GetMovement%20Component))
  (bind _dotdamage (Variables|Default|GetDOTDamage))
  (if (Utilities|DoesObjectImplementInterface (stale Custom|StartDOT AOEEffectOwner) "/Game/Player/BPI_Player.BPI_Player_C")
    (Class|BPIEnemy|TakeDamage(Message) _returnvalue _dotdamage (Variables|Default|GetEffectName))
    (switch name (Variables|Default|GetEffectName)
      (:Leeched
        (Class|BPIPlayer|Heal(Message) (stale Custom|StartDOT AOEEffectOwner) (Variables|Default|GetDOTDamage)))
      (:Slowed
        (Variables|/Script/Engine.CharacterMovementComponent|SetMaxWalkSpeed _movement_component (* (Variables|/Script/Engine.CharacterMovementComponent|GetMaxWalkSpeed _movement_component) 0.5))
        (Development|PrintString (Utilities|String|Append (Utilities|GetDisplayName (Components|GetOwner)) " IS SLOWED AND IS TAKING " (Utilities|String|ToString(Float) (Variables|Default|GetDOTDamage)) " EVERY " (Utilities|String|ToString(Float) (Variables|Default|GetDOTTick)) " SECONDS") true true "(R=0.488138,G=0.000000,B=1.000000,A=1.000000)" 1e+01 :!label _label)))
    (else
      (Class|BPIPlayer|TakeDamage(Message) _returnvalue _dotdamage)
      (switch name (Variables|Default|GetEffectName)
        (:Leeched
          (Class|BPIEnemy|Heal(Message) (stale Custom|StartDOT AOEEffectOwner) (Variables|Default|GetDOTDamage)))
        (:Slowed
          (Variables|/Script/Engine.CharacterMovementComponent|SetMaxWalkSpeed _movement_component (* (Variables|/Script/Engine.CharacterMovementComponent|GetMaxWalkSpeed _movement_component) 0.5))
          (goto _label))))))