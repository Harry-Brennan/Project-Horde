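; Actor component that provides a reusable damage calculation for its owning actor.
; TakeDamage checks a CanTakeDamage flag, then returns the passed-in health minus the damage, with no clamping.
; It prints the owner's name, the damage source and the new health to the screen.
; The component stores no health itself and has no active event logic.
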(event EventBeginPlay)

(event EventTick
  (params (DeltaSeconds :type Float%20%28single-precision%29)))

(fn TakeDamage
  (params (CurrentHealth :type Float%20%28double-precision%29) (DamageToTake :type Float%20%28double-precision%29) (CanTakeDamage :type Boolean) (DamageSource :type Name))
  (bind _returnvalue (Components|GetOwner))
  (bind _returnvalue_2 (- CurrentHealth DamageToTake))
  (bind _returnvalue_3 (Utilities|GetDisplayName _returnvalue))
  (if CanTakeDamage
    (Development|PrintString (Utilities|String|Append _returnvalue_3 " IS TAKING DAMAGE FROM : " (Utilities|String|ToString(Name) DamageSource)))
    (Development|PrintString (Utilities|String|Append _returnvalue_3 " IS NOW AT: " (Utilities|String|ToString(Float) _returnvalue_2) " HEALTH"))
    (return _returnvalue_2)))