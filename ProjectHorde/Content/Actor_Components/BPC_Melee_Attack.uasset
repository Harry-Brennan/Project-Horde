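; Actor component that gives its owner a melee attack, damaging pawns in front of it.
; MeleeAttack sweeps a sphere of the given radius from the owner's location a short fixed distance forward, ignoring the owner.
; Each hit actor receives a TakeDamageMessage with the given damage.
; It checks whether the owner implements BPI_Player, but both branches currently apply damage identically.
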(event EventBeginPlay)

(event EventTick
  (params (DeltaSeconds :type Float%20%28single-precision%29)))

(fn MeleeAttack
  (params (AreaSize :type Float%20%28double-precision%29) (Damage :type Float%20%28double-precision%29))
  (bind _returnvalue (Components|GetOwner))
  (bind _returnvalue_2 (Transformation|GetActorLocation _returnvalue))
  (bind _outhits (Collision|MultiSphereTraceForObjects _returnvalue_2 (+ _returnvalue_2 (* (Transformation|GetActorForwardVector _returnvalue) 1.5e+02)) AreaSize (Utilities|Array|MakeArray "ObjectTypeQuery3") false (Utilities|Array|MakeArray _returnvalue) "None"))
  (if (Utilities|DoesObjectImplementInterface (Components|GetOwner) "/Game/Player/BPI_Player.BPI_Player_C")
    (for _array_element _outhits
      (Class|BPIEnemy|TakeDamage(Message) (.HitActor (Collision|BreakHitResult _array_element)) Damage))
    (else
      (for _array_element_2 _outhits
        (Class|BPIPlayer|TakeDamage(Message) (.HitActor (Collision|BreakHitResult _array_element_2)) Damage)))))