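; Upgrade component that automatically fires poison bomb projectiles from its owning actor.
; A looping timer set on BeginPlay calls Shoot at the ReloadSpeed interval.
; Shoot spawns a BP_Projectile named PoisonBomb with the component's AOE radius, aimed horizontally toward random navmesh-reachable coordinates around the owner.
; UpgradePoisonBombStats is an empty stub.
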(event Custom|ShootLoop
  (CallFunction|Shoot))

(event EventBeginPlay
  (Utilities|Time|SetTimerbyEvent (delegate Custom|ShootLoop) (Variables|Default|GetReloadSpeed) true))

(fn Shoot
  (bind _returnvalue (Components|GetOwner))
  (bind _returnvalue_2 (Components|GetOwner))
  (bind _returnvalue_3 (Transformation|GetActorLocation _returnvalue))
  (bind _randomlocation (AI|Navigation|GetRandomReachablePointinRadius _returnvalue_3 1e+03 0 0))
  (Game|SpawnActorfromClass "/Game/Projectiles/BP_Projectile.BP_Projectile_C" (Math|Transform|MakeTransform (Transformation|GetActorLocation _returnvalue_2) (Math|Rotator|FindLookatRotation _returnvalue_3 (Math|Vector|MakeVector (.x _randomlocation) (.y _randomlocation) (.Z (Class|KismetMathLibrary|BreakVector3f _returnvalue_3)))) "1.000000,1.000000,1.000000") "AlwaysSpawn" "MultiplyWithRoot" _returnvalue_2 "PoisonBomb" 0.0 0.0 0.0 1.5e+02 0.0 (Variables|Default|GetAOERadius) 0))

(fn UpgradePoisonBombStats)