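; Pistol upgrade actor component that automatically fires for its owning actor on a repeating timer.
; BeginPlay starts a looping timer at ReloadSpeed, and each tick of it calls Shoot to spawn an actor at the owner's location, rotated along its velocity.
; UpgradePistol shortens ReloadSpeed by a tenth per call but does not restart the running timer.
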(event Custom|ShootLoop
  (CallFunction|Shoot))

(event EventBeginPlay
  (Utilities|Time|SetTimerbyEvent (delegate Custom|ShootLoop) (Variables|Default|GetReloadSpeed) true))

(fn Shoot
  (bind _returnvalue (Components|GetOwner))
  (Game|SpawnActorfromClass "/Game/Projectiles/BP_Projectile.BP_Projectile_C" (Math|Transform|MakeTransform (Transformation|GetActorLocation _returnvalue) (Math|Conversions|RotationFromXVector (Transformation|GetVelocity _returnvalue)) "1.000000,1.000000,1.000000") "AdjustIfPossibleButAlwaysSpawn" "MultiplyWithRoot" _returnvalue "PistolBullet" 0.0 0.0 0.0 1.5e+02 0))

(fn UpgradePistol
  (Variables|Default|SetReloadSpeed (* (Variables|Default|GetReloadSpeed) 0.9)))