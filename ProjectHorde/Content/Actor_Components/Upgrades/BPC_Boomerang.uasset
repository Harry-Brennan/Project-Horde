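; Upgrade component that gives its owner an automatic boomerang weapon, fired on a looping timer set by ReloadSpeed.
; Each shot spawns a BP_Projectile at the owner, aimed level toward a random reachable nearby point, then sets its speed and damage and starts its return timer.
; UpgradeBoomerangStats compounds the stats multiplicatively, shortening ReloadSpeed and raising speed and damage, but does not reset the running timer.
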(event Custom|ShootLoop
  (CallFunction|Shoot))

(event EventBeginPlay
  (Utilities|Time|SetTimerbyEvent (delegate Custom|ShootLoop) (Variables|Default|GetReloadSpeed) true))

(fn Shoot
  (bind _returnvalue (Components|GetOwner))
  (bind _returnvalue_2 (Components|GetOwner))
  (bind _returnvalue_3 (Transformation|GetActorLocation _returnvalue))
  (bind _randomlocation (AI|Navigation|GetRandomReachablePointinRadius _returnvalue_3 1e+03 0 0))
  (bind _returnvalue_4 (Game|SpawnActorfromClass "/Game/Projectiles/BP_Projectile.BP_Projectile_C" (Math|Transform|MakeTransform (Transformation|GetActorLocation _returnvalue_2) (Math|Rotator|FindLookatRotation _returnvalue_3 (Math|Vector|MakeVector (.x _randomlocation) (.y _randomlocation) (.Z (Class|KismetMathLibrary|BreakVector3f _returnvalue_3)))) "1.000000,1.000000,1.000000") "AdjustIfPossibleButAlwaysSpawn" "MultiplyWithRoot" _returnvalue_2 "Boomerang" 0.0 0.0 0.0 1.5e+02 (Variables|Default|GetTimeBeforeReturning) 0))
  (Variables|/Script/Engine.ProjectileMovementComponent|SetInitialSpeed (Variables|/Game/Projectiles/BP_Projectile.BP_Projectile_C|GetProjectileMovement _returnvalue_4) (* (Variables|/Game/Projectiles/BP_Projectile.BP_Projectile_C|GetBase%20Speed _returnvalue_4) (Variables|Default|GetBoomerangSpeedMultiplier)))
  (Variables|/Game/Projectiles/BP_Projectile.BP_Projectile_C|SetBase%20Damage _returnvalue_4 (Variables|Default|GetBoomerangDamage))
  (Default|StartReturningProjectileTimer _returnvalue_4))

(fn UpgradeBoomerangStats
  (Variables|Default|SetReloadSpeed (* (Variables|Default|GetReloadSpeed) 0.9))
  (Variables|Default|SetBoomerangSpeedMultiplier (* (Variables|Default|GetBoomerangSpeedMultiplier) 1.25))
  (Variables|Default|SetBoomerangDamage (* (Variables|Default|GetBoomerangDamage) 1.25)))