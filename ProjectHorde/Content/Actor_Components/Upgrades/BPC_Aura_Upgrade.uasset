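; Actor component upgrade that gives its owner a damage aura, periodically hurting nearby pawns.
; A looping timer set on BeginPlay runs a sphere trace around the owner, ignoring it, and sends a damage message to each hit actor.
; Owners implementing the player interface tag the damage with an "AURA" source, while others send damage alone.
; UpgradeAuraStats multiplicatively increases the aura's radius and damage.
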(event Custom|AuraHitCE
  (CallFunction|AuraHitDetection))

(event EventBeginPlay
  (Utilities|Time|SetTimerbyEvent (delegate Custom|AuraHitCE) (Variables|Default|GetAuraHitRate) true))

(fn AuraHitDetection
  (bind _returnvalue (Components|GetOwner))
  (bind _returnvalue_2 (Transformation|GetActorLocation _returnvalue))
  (bind _outhits (Collision|MultiSphereTraceForObjects _returnvalue_2 _returnvalue_2 (Variables|Default|GetAuraRadius) (Utilities|Array|MakeArray "ObjectTypeQuery3") false (Utilities|Array|MakeArray _returnvalue) "ForOneFrame"))
  (if (Utilities|DoesObjectImplementInterface (Components|GetOwner) "/Game/Player/BPI_Player.BPI_Player_C")
    (for _array_element _outhits
      (Class|BPIEnemy|TakeDamage(Message) (.HitActor (Collision|BreakHitResult _array_element)) (Variables|Default|GetAuraDamage) "AURA"))
    (else
      (for _array_element_2 _outhits
        (Class|BPIPlayer|TakeDamage(Message) (.HitActor (Collision|BreakHitResult _array_element_2)) (Variables|Default|GetAuraDamage))))))

(fn UpgradeAuraStats
  (Variables|Default|SetAuraRadius (* (Variables|Default|GetAuraRadius) 1.5))
  (Variables|Default|SetAuraDamage (* (Variables|Default|GetAuraDamage) 1.25)))