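; Upgrade component that makes its owner periodically fire an explosive bomb projectile at a target.
; A fast looping timer refreshes the target: the player's closest enemy if the owner implements BPI_Player, otherwise the player character.
; A second timer spawns BP_Projectile aimed at that target, passing radius and damage.
; UpgradeBombStats scales reload, damage and radius, but the running fire timer keeps its original interval.
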(event Custom|ShootingBombTimer
  (CallFunction|ShootBomb))

(event Custom|UpdateClosestEnemy
  (bind _returnvalue (Game|GetPlayerCharacter 0))
  (if (Utilities|DoesObjectImplementInterface (Components|GetOwner) "/Game/Player/BPI_Player.BPI_Player_C")
    (bind _closestenemy (Class|BPIPlayer|GetClosestEnemy(Message) _returnvalue))
    (Variables|Default|SetClosestEnemy _closestenemy)
    (else
      (Variables|Default|SetClosestEnemy _returnvalue))))

(event EventBeginPlay
  (Utilities|Time|SetTimerbyEvent (delegate Custom|ShootingBombTimer) (Variables|Default|GetBombReloadSpeed) true)
  (Utilities|Time|SetTimerbyEvent (delegate Custom|UpdateClosestEnemy) 0.1 true))

(fn ShootBomb
  (bind _returnvalue (Components|GetOwner))
  (Game|SpawnActorfromClass "/Game/Projectiles/BP_Projectile.BP_Projectile_C" (Math|Transform|MakeTransform (Transformation|GetActorLocation _returnvalue) (Math|Rotator|FindLookatRotation (Transformation|GetActorLocation (Components|GetOwner)) (Transformation|GetActorLocation (Variables|Default|GetClosestEnemy))) "1.000000,1.000000,1.000000") "AdjustIfPossibleButAlwaysSpawn" "MultiplyWithRoot" _returnvalue "Bomb" (Variables|Default|GetBombAOERadius) (Variables|Default|GetBombDamage) 0))

(fn UpgradeBombStats
  (Variables|Default|SetBombReloadSpeed (* (Variables|Default|GetBombReloadSpeed) 0.9))
  (Variables|Default|SetBombDamage (* (Variables|Default|GetBombDamage) 1.25))
  (Variables|Default|SetBombAOERadius (* (Variables|Default|GetBombAOERadius) 1.25)))