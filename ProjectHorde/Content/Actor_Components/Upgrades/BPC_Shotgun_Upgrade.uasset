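; Shotgun upgrade component that automatically fires spread volleys from its owning actor.
; A looping timer, set once on BeginPlay from ReloadSpeed, calls Shoot for each pellet.
; Each shot spawns an actor at the owner's location, facing its velocity direction with random yaw spread.
; UpgradeShotgun adds pellets and shortens ReloadSpeed, but does not reset the running timer.
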(event Custom|ShootLoop
  (for _index (range 1 (Variables|Default|GetNumberOfPellets))
    (CallFunction|Shoot)))

(event EventBeginPlay
  (Utilities|Time|SetTimerbyEvent (delegate Custom|ShootLoop) (Variables|Default|GetReloadSpeed) true))

(fn Shoot
  (bind _returnvalue (Components|GetOwner))
  (bind _returnvalue_2 (Transformation|GetVelocity _returnvalue))
  (bind _returnvalue_3 (Math|Conversions|RotationFromXVector _returnvalue_2))
  (Game|SpawnActorfromClass "/Game/Projectiles/BP_Projectile.BP_Projectile_C" (Math|Transform|MakeTransform (Transformation|GetActorLocation _returnvalue) (Math|Rotator|MakeRotator (.roll _returnvalue_3) (.pitch _returnvalue_3) (+ (.yaw _returnvalue_3) (Math|Random|RandomFloatinRange -5.0 5.0))) "1.000000,1.000000,1.000000") "AdjustIfPossibleButAlwaysSpawn" "MultiplyWithRoot" _returnvalue "ShotgunPellet" 0.0 0.0 0.0 1.5e+02 0))

(fn UpgradeShotgun
  (Variables|Default|SetNumberOfPellets (+ (Variables|Default|GetNumberOfPellets) 2))
  (Variables|Default|SetReloadSpeed (* (Variables|Default|GetReloadSpeed) 0.9)))