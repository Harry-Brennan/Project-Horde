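; Upgrade component that gives its owning actor a scythe projectile that rotates around it.
; On BeginPlay it spawns a BP_Projectile just in front of the owner with the component's RotatingRadius, stores it and starts its rotation.
; UpgradeScytheStats raises the projectile's base damage and scales down its RotatingRate, but enlarges only the component's RotatingRadius, without passing it to the spawned projectile.
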(event EventBeginPlay
  (bind _returnvalue (Components|GetOwner))
  (bind _returnvalue_2 (Game|SpawnActorfromClass "/Game/Projectiles/BP_Projectile.BP_Projectile_C" (Math|Transform|MakeTransform (+ (Transformation|GetActorLocation _returnvalue) (* (Transformation|GetActorForwardVector _returnvalue) 5e+01)) "0, 0, 0" "1.000000,1.000000,1.000000") "AdjustIfPossibleButAlwaysSpawn" "MultiplyWithRoot" (Components|GetOwner) "Scythe" 0.0 0.0 0.0 (Variables|Default|GetRotatingRadius) 0))
  (bind _output_get (Variables|Default|SetSpawnedScytheProjectile _returnvalue_2))
  (Default|RotateProjectileAroundOwner _output_get))

(fn UpgradeScytheStats
  (bind _spawnedscytheprojectile (Variables|Default|GetSpawnedScytheProjectile))
  (bind _spawnedscytheprojectile_2 (Variables|Default|GetSpawnedScytheProjectile))
  (Variables|/Game/Projectiles/BP_Projectile.BP_Projectile_C|SetBase%20Damage _spawnedscytheprojectile_2 (* (Variables|/Game/Projectiles/BP_Projectile.BP_Projectile_C|GetBase%20Damage _spawnedscytheprojectile_2) 1.25))
  (Variables|Default|SetRotatingRadius (* (Variables|Default|GetRotatingRadius) 1.5))
  (Variables|/Game/Projectiles/BP_Projectile.BP_Projectile_C|SetRotatingRate _spawnedscytheprojectile (* (Variables|/Game/Projectiles/BP_Projectile.BP_Projectile_C|GetRotatingRate _spawnedscytheprojectile) 0.75)))