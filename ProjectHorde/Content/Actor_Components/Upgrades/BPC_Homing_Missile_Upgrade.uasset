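; Upgrade component that periodically fires homing missiles from its owning actor.
; A looping timer set on BeginPlay spawns a BP_Projectile at the owner, yawed toward random reachable nearby points, passes in explosion and homing stats, then starts homing.
; UpgradeMissileStats scales reload, damage, blast radius and homing strength multiplicatively.
; The timer is never reset, so reload upgrades leave the running interval unchanged.
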(event Custom|ShootHomingMissile
  (CallFunction|ShootMissile))

(event EventBeginPlay
  (Utilities|Time|SetTimerbyEvent (delegate Custom|ShootHomingMissile) (Variables|Default|GetMissileReloadSpeed) true))

(fn ShootMissile
  (bind _returnvalue (Components|GetOwner))
  (bind _returnvalue_2 (Components|GetOwner))
  (bind _returnvalue_3 (Transformation|GetActorLocation _returnvalue))
  (bind _randomlocation (AI|Navigation|GetRandomReachablePointinRadius _returnvalue_3 1e+03 0 0))
  (bind _returnvalue_4 (Game|SpawnActorfromClass "/Game/Projectiles/BP_Projectile.BP_Projectile_C" (Math|Transform|MakeTransform (Transformation|GetActorLocation _returnvalue_2) (Math|Rotator|FindLookatRotation _returnvalue_3 (Math|Vector|MakeVector (.x _randomlocation) (.y _randomlocation) (.Z (Class|KismetMathLibrary|BreakVector3f _returnvalue_3)))) "1.000000,1.000000,1.000000") "AdjustIfPossibleButAlwaysSpawn" "MultiplyWithRoot" _returnvalue_2 "HomingMissile" (Variables|Default|GetMissileAOERadius) (Variables|Default|GetMissileDamage) (Variables|Default|GetMissileHomingStrength) 1.5e+02 0))
  (Default|StartHoming _returnvalue_4))

(fn UpgradeMissileStats
  (Variables|Default|SetMissileReloadSpeed (* (Variables|Default|GetMissileReloadSpeed) 0.9))
  (Variables|Default|SetMissileDamage (* (Variables|Default|GetMissileDamage) 1.25))
  (Variables|Default|SetMissileAOERadius (* (Variables|Default|GetMissileAOERadius) 1.25))
  (Variables|Default|SetMissileHomingStrength (* (Variables|Default|GetMissileHomingStrength) 1.5)))